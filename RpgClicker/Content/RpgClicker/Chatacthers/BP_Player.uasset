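; Player character Blueprint for an RPG clicker that holds the player's money and handles death.
; Money gets a starting balance on BeginPlay, with events to add or subtract it (clamped at zero) and functions to check it or attempt a purchase.
; On death, it has GM_Gameplay take away money, then restores health to maximum instead of destroying the player.
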(event Custom|DecreaseMoney
  (params (Amount :type Integer))
  (Variables|Default|SetMoney (- (Variables|Default|GetMoney) Amount))
  (if (< (Variables|Default|GetMoney) 0)
    (Variables|Default|SetMoney 0)))

(event Custom|RecoverAllHP
  (bind _returnvalue (Class|BaseCharacter|GetMaxHealth))
  (Class|BaseCharacter|SetHealth _returnvalue))

(event Custom|IncreaseMoney
  (params (Amount :type Integer))
  (Variables|Default|SetMoney (+ (Variables|Default|GetMoney) Amount)))

(event EventBeginPlay
  (Variables|Default|SetMoney 1500))

(event Collision|EventActorBeginOverlap
  (params (OtherActor :type Actor%20Object%20Reference)))

(event EventOnDeath
  (bind _asgm_gameplay (Utilities|Casting|CastToGM_Gameplay (Game|GetGameMode)))
  (Default|TakeAwayMoney _asgm_gameplay)
  (CallFunction|RecoverAllHP))

(fn ConstructionScript)

(fn AttemptBuy
  (params (Price :type Integer))
  (if (>= (Variables|Default|GetMoney) Price)
    (Variables|Default|SetMoney (- (Variables|Default|GetMoney) Price))
    (return true)
    (else
      (return false))))

(fn HasMoney
  (return (> (Variables|Default|GetMoney) 0)))