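; BP_Enemy is the enemy in an RPG clicker, which rolls random combat stats scaled by the game's threat level.
; On BeginPlay it reads TreathLevel from GM_Gameplay to randomize attack, defense, avoid, crit and max health, then refills health.
; On death the same actor rerolls instead of being destroyed, then tells the game mode to pay the player and raise the threat, so each reroll uses the pre-increase level.
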(event Custom|Generate%20random%20stats
  (bind _asgm_gameplay (Utilities|Casting|CastToGM_Gameplay (Game|GetGameMode)))
  (Class|BaseCharacter|SetAttack (+ (Variables|/Game/RpgClicker/GameModes/GM_Gameplay.GM_Gameplay_C|GetTreathLevel _asgm_gameplay) (Math|Random|RandomIntegerinRange 4 10)))
  (Class|BaseCharacter|SetDefense (+ (Math|Random|RandomIntegerinRange 5 7) (Variables|/Game/RpgClicker/GameModes/GM_Gameplay.GM_Gameplay_C|GetTreathLevel _asgm_gameplay)))
  (Class|BaseCharacter|SetAvoidChance (Math|Random|RandomIntegerinRange (Variables|/Game/RpgClicker/GameModes/GM_Gameplay.GM_Gameplay_C|GetTreathLevel _asgm_gameplay) 50))
  (Class|BaseCharacter|SetCritChance (Math|Random|RandomIntegerinRange (Variables|/Game/RpgClicker/GameModes/GM_Gameplay.GM_Gameplay_C|GetTreathLevel _asgm_gameplay) 50))
  (Class|BaseCharacter|SetMaxHealth (+ (Math|Random|RandomIntegerinRange 20 200) (Variables|/Game/RpgClicker/GameModes/GM_Gameplay.GM_Gameplay_C|GetTreathLevel _asgm_gameplay)))
  (bind _returnvalue (Class|BaseCharacter|GetMaxHealth))
  (Class|BaseCharacter|SetHealth _returnvalue))

(event EventBeginPlay
  (CallFunction|GenerateRandomStats))

(event Collision|EventActorBeginOverlap
  (params (OtherActor :type Actor%20Object%20Reference)))

(event EventTick
  (params (DeltaSeconds :type Float%20%28single-precision%29)))

(event EventOnDeath
  (Development|PrintString "I AM DEAD")
  (CallFunction|GenerateRandomStats)
  (bind _asgm_gameplay (Utilities|Casting|CastToGM_Gameplay (Game|GetGameMode)))
  (Default|GivePlayerMoney _asgm_gameplay)
  (Default|RaiseTreathLevel _asgm_gameplay))

(fn ConstructionScript)