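; Gameplay game mode for an RPG clicker that spawns the player and enemy, shows the gameplay widget and drives each attack exchange.
; A threat level scales money gains, losses and stat increases, all routed through the player controller and its player reference.
; Shop prices double per purchase type, and taking money from a player who has none triggers game over and returns to the main menu.
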(event Custom|GivePlayerMoney
  (bind _asbp_player_controller (Utilities|Casting|CastToBP_PlayerController (Game|GetPlayerController 0)))
  (Default|IncreaseMoney _asbp_player_controller (* (Variables|Default|GetMoneyGainBase) (Variables|Default|GetTreathLevel))))

(event Custom|OnAttack
  (bind _asbp_player_controller (Utilities|Casting|CastToBP_PlayerController (Game|GetPlayerController 0)))
  (Default|Attack _asbp_player_controller (Variables|Default|GetEnemy))
  (Class|BaseCharacter|PerformAttack (Variables|Default|GetEnemy) (Variables|Default|GetPlayer)))

(event Custom|TakeAwayMoney
  (bind _asbp_player_controller (Utilities|Casting|CastToBP_PlayerController (Game|GetPlayerController 0)))
  (bind _result (Default|HasMoney (Variables|/Game/RpgClicker/Chatacthers/BP_PlayerController.BP_PlayerController_C|GetPlayerRef _asbp_player_controller)))
  (if _result
    (Default|DecreaseMoney (Variables|/Game/RpgClicker/Chatacthers/BP_PlayerController.BP_PlayerController_C|GetPlayerRef _asbp_player_controller) (* (Variables|Default|GetMoneyGainBase) (Variables|Default|GetTreathLevel)))
    (else
      (CallFunction|OnGameOver))))

(event Custom|OnGameOver
  (Development|PrintString "GameOver...")
  (Game|OpenLevel(byObjectReference) "/Game/RpgClicker/Maps/M_MainMenu.M_MainMenu"))

(event Custom|Raise%20TreathLevel
  (bind _result (Math|Integer|IncrementInt (Variables|Default|GetTreathLevel))
    (:%20%20
      (Variables|Default|SetTreathLevel _result))))

(event EventBeginPlay
  (Variables|Default|SetTreathLevel 1)
  (bind _returnvalue (Game|SpawnActorfromClass "/Game/RpgClicker/Chatacthers/BP_Player.BP_Player_C" (Math|Transform|MakeTransform "0, 0, 0") "Undefined" 0 0 0))
  (Variables|Default|SetPlayer _returnvalue)
  (bind _asbp_player_controller (Utilities|Casting|CastToBP_PlayerController (Game|GetPlayerController 0))
    (:then
      (Variables|/Game/RpgClicker/Chatacthers/BP_PlayerController.BP_PlayerController_C|SetPlayerRef _asbp_player_controller (Variables|Default|GetPlayer))
      (bind _returnvalue_2 (Game|SpawnActorfromClass "/Game/RpgClicker/Chatacthers/BP_Enemy.BP_Enemy_C" (Math|Transform|MakeTransform "0, 0, 0") "Undefined" 0 0))
      (Variables|Default|SetEnemy _returnvalue_2)
      (bind _returnvalue_3 (UserInterface|CreateWidget "/Game/RpgClicker/UI/WBP_Gameplay.WBP_Gameplay_C"))
      (UserInterface|Viewport|AddtoViewport _returnvalue_3 0)
      (Variables|/Script/Engine.PlayerController|SetbShowMouseCursor (Game|GetPlayerController 0) true))
    (:CastFailed
      (Development|PrintString "Skrrr"))))

(fn ConstructionScript)

(fn RaisePrice
  (params (PriceType :type E_PriceType%20Enum :default "NewEnumerator0"))
  (switch Utilities|FlowControl|Switch|SwitchonE_PriceType PriceType
    (:NewEnumerator0
      (Variables|Default|SetHealPrice (* (Variables|Default|GetHealPrice) 2)))
    (:NewEnumerator1
      (Variables|Default|SetSwordPrice (* (Variables|Default|GetSwordPrice) 2)))
    (:NewEnumerator2
      (Variables|Default|SetArmorPrice (* (Variables|Default|GetArmorPrice) 2)))
    (:NewEnumerator3
      (Variables|Default|SetPrecisionPrice (* (Variables|Default|GetPrecisionPrice) 2)))
    (:NewEnumerator4
      (Variables|Default|SetEvasionPrice (* (Variables|Default|GetEvasionPrice) 2)))))

(fn RaiseStat
  (params (Type :type E_StatType%20Enum :default "NewEnumerator0"))
  (bind _treathlevel (Variables|Default|GetTreathLevel))
  (bind _asbp_player_controller (Utilities|Casting|CastToBP_PlayerController (Game|GetPlayerController 0)))
  (switch Utilities|FlowControl|Switch|SwitchonE_StatType Type
    (:NewEnumerator0
      (bind _returnvalue (Class|BaseCharacter|GetAttack (Variables|/Game/RpgClicker/Chatacthers/BP_PlayerController.BP_PlayerController_C|GetPlayerRef _asbp_player_controller)))
      (Class|BaseCharacter|SetAttack (Variables|/Game/RpgClicker/Chatacthers/BP_PlayerController.BP_PlayerController_C|GetPlayerRef _asbp_player_controller) (+ _returnvalue _treathlevel)))
    (:NewEnumerator1
      (bind _returnvalue_2 (Class|BaseCharacter|GetDefense (Variables|/Game/RpgClicker/Chatacthers/BP_PlayerController.BP_PlayerController_C|GetPlayerRef _asbp_player_controller)))
      (Class|BaseCharacter|SetDefense (Variables|/Game/RpgClicker/Chatacthers/BP_PlayerController.BP_PlayerController_C|GetPlayerRef _asbp_player_controller) (+ _returnvalue_2 _treathlevel)))
    (:NewEnumerator2
      (bind _returnvalue_3 (Class|BaseCharacter|GetAvoidChance (Variables|/Game/RpgClicker/Chatacthers/BP_PlayerController.BP_PlayerController_C|GetPlayerRef _asbp_player_controller)))
      (Class|BaseCharacter|SetAvoidChance (Variables|/Game/RpgClicker/Chatacthers/BP_PlayerController.BP_PlayerController_C|GetPlayerRef _asbp_player_controller) (+ _returnvalue_3 _treathlevel)))
    (:NewEnumerator3
      (bind _returnvalue_4 (Class|BaseCharacter|GetCritChance (Variables|/Game/RpgClicker/Chatacthers/BP_PlayerController.BP_PlayerController_C|GetPlayerRef _asbp_player_controller)))
      (Class|BaseCharacter|SetCritChance (Variables|/Game/RpgClicker/Chatacthers/BP_PlayerController.BP_PlayerController_C|GetPlayerRef _asbp_player_controller) (+ _returnvalue_4 _treathlevel)))))